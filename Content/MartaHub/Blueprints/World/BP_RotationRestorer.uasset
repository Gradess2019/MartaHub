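; BP_RotationRestorer is an actor component that smoothly returns its owner to the rotation it had at BeginPlay.
; Restore turns off the owner's movement replication and calls MulticastRestore, which records the current rotation and enables component tick.
; Tick interpolates along the shortest path for about one second, then resets its timer, disables tick and calls OnFinished.
; Movement replication is not re-enabled within this component.
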(event `self.ReceiveBeginPlay`
  (set `self.InitialRotation` (`Actor.K2_GetActorRotation` (`self.GetOwner`))))

(event `self.Restore`
  (`Actor.SetReplicateMovement` (`self.GetOwner`) false)
  (`self.MulticastRestore`))

(event `MulticastRestore`
  (`self.SetComponentTickEnabled` true)
  (set `self.StartRotation` (`Actor.K2_GetActorRotation` (`self.GetOwner`))))

(event `self.ReceiveTick`
  (params (DeltaSeconds :type "Float (single-precision)"))
  (set `self.ElapsedTime` (+ DeltaSeconds (`self.ElapsedTime`)))
  (`Actor.K2_SetActorRotation` (`self.GetOwner`) (`KismetMathLibrary.RLerp` (`self.StartRotation`) (`self.InitialRotation`) (`self.ElapsedTime`) true) false)
  (if (>= (`self.ElapsedTime`) 1.0)
    (set `self.ElapsedTime` 0.0)
    (`self.SetComponentTickEnabled` false)
    (`self.OnFinished`)))