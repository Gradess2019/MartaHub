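; Networked pickupable radio prop that can be carried, thrown (including on damage), highlighted via custom depth and given an initial volume by the server.
; Pickup and throw events forward to a Pickupable component, while Interact opens a radio options window bound to this actor through a CreateWidgetCommand.
; Server-side Restore pauses movement replication while location and rotation restorers run, re-enabling it when either completes.
; It also exposes its SnapshotManager.
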(event `self.ReceiveBeginPlay`
  (`parent.ReceiveBeginPlay`)
  (`/Engine/EditorBlueprintResources/ActorMacros.Switch Has Authority`
    (:`Authority`
      (`KismetSystemLibrary.Delay` 0.2)
      (`self.SetVolume` (`self.InitialVolume`)))))

(event `self.PreparePickup`
  (message `Pickupable.PreparePickup` (`self.Pickupable`)))

(event `self.Throw`
  (params (Force :type "Float (single-precision)"))
  (message `Pickupable.Throw` (`self.Pickupable`) Force))

(event `self.ClearPickup`
  (message `Pickupable.ClearPickup` (`self.Pickupable`)))

(event `self.ReceiveAnyDamage`
  (params (Damage :type "Float (single-precision)") (DamageType :type "DamageType Object Reference") (InstigatedBy :type "Controller Object Reference") (DamageCauser :type "Actor Object Reference"))
  (`self.Throw` Damage))

(event `self.SetPickupLocation`
  (params (OwnerLocation :type "Vector Structure (by ref)") (OwnerDirection :type "Vector Structure (by ref)"))
  (message `Pickupable.SetPickupLocation` (`self.Pickupable`) OwnerLocation OwnerDirection))

(event `self.Restore`
  (`/Engine/EditorBlueprintResources/ActorMacros.Switch Has Authority`
    (:`Authority`
      (`self.SetReplicateMovement` false)
      (message `Restorer.Restore` (`self.LocationRestorer`))
      (message `Restorer.Restore` (`self.RotationRestorer`)))))

(event `self.LocationRestorer.OnRestoringComplete`
  (`/Engine/EditorBlueprintResources/ActorMacros.Switch Has Authority` :!label _label
    (:`Authority`
      (`self.SetReplicateMovement` true))))

(event `self.RotationRestorer.OnRestoringComplete`
  (goto _label))

(event `self.Select`
  (`PrimitiveComponent.SetRenderCustomDepth` (`self.StaticMeshComponent`) true))

(event `self.Unselect`
  (`PrimitiveComponent.SetRenderCustomDepth` (`self.StaticMeshComponent`) false))

(event `self.Interact`
  (bind _returnvalue (`|GenericCreateObject` "/Script/CommandPack.CreateWidgetCommand" self))
  (bind _returnvalue_2 (`CreateWidgetCommand.Init` _returnvalue (make `CreateWidgetCommandData` (`GameplayStatics.GetPlayerController` 0) "/Game/MartaHub/Blueprints/Widgets/Windows/WBP_RadioOptionsWindow.WBP_RadioOptionsWindow_C")))
  (if _returnvalue_2
    (`BaseCommand.Execute` _returnvalue)
    (bind (_bsuccess _returnvalue_3) (`CreateWidgetCommand.GetWidget` _returnvalue))
    (bind _aswbp_radio_options_window (cast `/Game/MartaHub/Blueprints/Widgets/Windows/WBP_RadioOptionsWindow` _returnvalue_3))
    (`/Game/MartaHub/Blueprints/Widgets/Windows/WBP_RadioOptions.Init` (`/Game/MartaHub/Blueprints/Widgets/Windows/WBP_RadioOptionsWindow.WBP_RadioOptions` _aswbp_radio_options_window) self)))

(fn `GetSnapshotManager`
  (returns (ReturnValue :type "SnapshotManager Interface"))
  (return (`self.SnapshotManager`)))

(fn `UserConstructionScript`
  (`parent.UserConstructionScript`))