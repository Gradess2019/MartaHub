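; BP_PhysicalActor is a physics prop that can be picked up and thrown, with mesh and mass loaded from a data asset at construction.
; Pickup, placement and throw events forward to its Pickupable, and any damage taken also triggers a throw using the damage as force.
; Hits above a velocity threshold play a wood sound, throttled by a randomly delayed DoOnce reset, with volume scaled by mass and a Power parameter by speed.
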(event `self.ReceiveAnyDamage`
  (params (Damage :type "Float (single-precision)") (DamageType :type "DamageType Object Reference") (InstigatedBy :type "Controller Object Reference") (DamageCauser :type "Actor Object Reference"))
  (`self.Throw` Damage))

(event `self.StaticMeshComponent.OnComponentHit`
  (params (HitComponent :type "PrimitiveComponent Object Reference") (OtherActor :type "Actor Object Reference") (OtherComp :type "PrimitiveComponent Object Reference") (NormalImpulse :type "Vector Structure") (Hit :type "HitResult Structure (by ref)"))
  (`self.PlayHitSound` Hit))

(event `PlayHitSound`
  (params (Hit :type "HitResult Structure (by ref)"))
  (`|ExecutionSequence`
    (:`then_0`
      (`/Engine/EditorBlueprintResources/StandardMacros.DoOnce` false :!label _label
        (:`Completed`
          (if (> (`KismetMathLibrary.VSizeSquared` (`self.GetVelocity`)) (`self.VelocitySoundThreshold`))
            (`self.SpawnHitSound` Hit)))))
    (:`then_1`
      (`KismetSystemLibrary.Delay` (`KismetMathLibrary.RandomFloatInRange` 0.1 0.2))
      (goto _label :!via `Reset`))))

(event `self.PreparePickup`
  (message `Pickupable.PreparePickup` (`self.Pickupable`)))

(event `self.Throw`
  (params (Force :type "Float (single-precision)"))
  (message `Pickupable.Throw` (`self.Pickupable`) Force))

(event `self.ClearPickup`
  (message `Pickupable.ClearPickup` (`self.Pickupable`)))

(event `self.SetPickupLocation`
  (params (OwnerLocation :type "Vector Structure (by ref)") (OwnerDirection :type "Vector Structure (by ref)"))
  (message `Pickupable.SetPickupLocation` (`self.Pickupable`) OwnerLocation OwnerDirection))

(fn `ConvertVelocityToPower`
  (returns (ReturnValue :type Integer))
  (locals (NumOfParams :type Integer :default 3))
  (bind _velocitysoundthreshold (`self.VelocitySoundThreshold`))
  (return (`KismetMathLibrary.Round` (`KismetMathLibrary.MapRangeClamped` (`KismetMathLibrary.VSizeSquared` (`self.GetVelocity`)) _velocitysoundthreshold (* (`local.NumOfParams`) _velocitysoundthreshold) 0.0 2.0))))

(fn `LoadDataAsset`
  (`/Engine/EditorBlueprintResources/StandardMacros.IsValid` (`self.DataAsset`)
    (:`Is Valid`
      (`PrimitiveComponent.SetMassOverrideInKg` (`self.StaticMeshComponent`) "None" (`PhysicalActorInfo.Mass` (`self.DataAsset`)) true)
      (`StaticMeshComponent.SetStaticMesh` (`self.StaticMeshComponent`) (`PhysicalActorInfo.Mesh` (`self.DataAsset`))))))

(fn `SpawnHitSound`
  (params (Hit :type "HitResult Structure (by ref)"))
  (bind _returnvalue (`GameplayStatics.SpawnSoundAtLocation` "/Game/MartaHub/Sounds/Actors/Hit/A_WoodHit_Cue.A_WoodHit_Cue" (`.Location` (`GameplayStatics.BreakHitResult` Hit)) (struct) (`KismetMathLibrary.MapRangeClamped` (`PrimitiveComponent.GetMass` (`self.StaticMeshComponent`)) 0.0 30.0 0.2 3.0) 1.0 0.0 null null))
  (`/Engine/EditorBlueprintResources/StandardMacros.IsValid` _returnvalue
    (:`Is Valid`
      (`AudioComponent.SetIntParameter` _returnvalue "Power" (`self.ConvertVelocityToPower`)))))

(fn `UserConstructionScript`
  (`self.LoadDataAsset`))