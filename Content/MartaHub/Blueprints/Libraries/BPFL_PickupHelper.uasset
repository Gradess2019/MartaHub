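; BPFL_PickupHelper is a Blueprint function library of transform math for placing a picked-up target in front of its owner.
; CalculateLerpLocation blends the target's location toward a point at Bound along the owner's direction, plus an offset from the owner's location.
; CalculateLocation reuses it with full alpha to return that hold point directly.
; CalculateLerpRotation blends the target's rotation toward the owner's direction along the shortest path.
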(fn `CalculateLerpLocation`
  (params (Target :type "Actor Object Reference") (OwnerLocation :type "Vector Structure") (OwnerDirection :type "Vector Structure") (Offset :type "Vector Structure") (Bound :type "Float (double-precision)") (Alpha :type "Float (double-precision)"))
  (returns (ReturnValue :type "Vector Structure"))
  (return (`KismetMathLibrary.VLerp` (`Actor.K2_GetActorLocation` Target) (+ (* (`local.OwnerDirection`) (`local.Bound`)) (`local.OwnerLocation`) (`local.Offset`)) (`local.Alpha`))))

(fn `CalculateLerpRotation`
  (params (Target :type "Actor Object Reference") (OwnerDirection :type "Vector Structure") (Alpha :type "Float (double-precision)"))
  (returns (ReturnValue :type "Rotator Structure"))
  (return (`KismetMathLibrary.RLerp` (`Actor.K2_GetActorRotation` Target) (`KismetMathLibrary.Conv_VectorToRotator` (`local.OwnerDirection`)) (`local.Alpha`) true)))

(fn `CalculateLocation`
  (params (Target :type "Actor Object Reference") (OwnerLocation :type "Vector Structure") (OwnerDirection :type "Vector Structure") (Offset :type "Vector Structure") (Bound :type "Float (double-precision)"))
  (returns (ReturnValue :type "Vector Structure"))
  (return (`self.CalculateLerpLocation` Target OwnerLocation OwnerDirection Offset Bound 1.0 (`local.__WorldContext`))))