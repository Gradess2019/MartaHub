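; BP_PickupStateBase is the base object for pickup states, holding a reference to an owner and the picked-up actor.
; InitData stores both references and can register the state on the owner through SetPickupStateMessage.
; InitDataByState copies the same data from another state, so context can carry over from one state to the next.
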(fn `InitData`
  (params (Owner :type "SceneComponent Object Reference") (PickupedActor :type "Actor Object Reference") (bUpdateOwner :type Boolean :default true))
  (set `self.Owner` Owner)
  (set `self.PickupedActor` PickupedActor)
  (if (`local.bUpdateOwner`)
    (message `/Game/MartaHub/Blueprints/Interfaces/BPI_Pickuper.SetPickupState` (`self.Owner`) self)))

(fn `InitDataByState`
  (params (OtherState :type "/Game/MartaHub/Blueprints/States/BP_PickupStateBase Object Reference") (bUpdateOwner :type Boolean))
  (`self.InitData` (`/Game/MartaHub/Blueprints/States/BP_PickupStateBase.Owner` OtherState) (`/Game/MartaHub/Blueprints/States/BP_PickupStateBase.PickupedActor` OtherState) bUpdateOwner))