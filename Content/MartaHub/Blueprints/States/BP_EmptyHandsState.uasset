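; Empty-hands state in an interaction state machine, handling pickup of physical actors.
; On interact, it line-traces 200 units forward from its owner for PhysicsBody objects and continues only if it hits a BP_PhysicalActor.
; It prepares that actor for pickup, directly in standalone or through a multicast otherwise.
; It then constructs a BP_BusyHandsState initialized from itself, with the owner update flag set.
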(event `self.PressInteract`
  (bind _pickupedactor (`self.PickupedActor`))
  (bind _asbp_physical_actor (cast `/Game/MartaHub/Blueprints/World/BP_PhysicalActor` (`.HitActor` (`GameplayStatics.BreakHitResult` (`self.DoLineTrace`)))))
  (set `self.PickupedActor` _asbp_physical_actor)
  (if (`KismetSystemLibrary.IsStandalone`)
    (`/Game/MartaHub/Blueprints/World/BP_PhysicalActor.PrepareForPickup` _pickupedactor)
    (else
      (`/Game/MartaHub/Blueprints/World/BP_PhysicalActor.Multicast_PrepareForPickup` _pickupedactor)))
  (bind _returnvalue (`|GenericCreateObject` "/Game/MartaHub/Blueprints/States/BP_BusyHandsState.BP_BusyHandsState_C" (`self.Owner`)))
  (`self.InitDataByState` _returnvalue self true))

(fn `DoLineTrace`
  (returns (Hit :type "HitResult Structure") (ReturnValue :type Boolean))
  (bind _returnvalue (`SceneComponent.K2_GetComponentLocation` (`self.Owner`)))
  (bind (_outhit _returnvalue_2) (`KismetSystemLibrary.LineTraceSingleForObjects` _returnvalue (+ _returnvalue (* (`SceneComponent.GetForwardVector` (`self.Owner`)) 200.0)) (`|MakeArray` "ObjectTypeQuery4" :!type "EObjectTypeQuery Enum")))
  (return _outhit _returnvalue_2))