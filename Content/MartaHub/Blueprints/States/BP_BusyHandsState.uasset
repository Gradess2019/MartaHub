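; BP_BusyHandsState is the hand state used while the owner carries a picked-up actor.
; Each update moves the carried actor to follow the owner's location and forward direction.
; Fire drops it and applies heavy damage to it, while releasing interact just drops it, using a server call outside standalone play.
; Both then switch to a new BP_EmptyHandsState initialized from this state, forming a state-object pattern.
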(event `self.Update`
  (params (DeltaTime :type "Float (single-precision)"))
  (bind _owner (`self.Owner`))
  (`/Game/MartaHub/Blueprints/World/BP_PhysicalActor.SetPickupLocation` (`self.PickupedActor`) (`SceneComponent.K2_GetComponentLocation` _owner) (`SceneComponent.GetForwardVector` _owner)))

(event `self.PressFire`
  (`self.ClearPickup`)
  (`GameplayStatics.ApplyDamage` (`self.PickupedActor`) 1000.0)
  (`self.SetNextState` :!label _label))

(event `self.ReleaseInteract`
  (`self.ClearPickup`)
  (goto _label))

(fn `ClearPickup`
  (bind _pickupedactor (`self.PickupedActor`))
  (if (`KismetSystemLibrary.IsStandalone`)
    (`/Game/MartaHub/Blueprints/World/BP_PhysicalActor.ClearPickup` _pickupedactor)
    (else
      (`/Game/MartaHub/Blueprints/World/BP_PhysicalActor.Server_ClearPickup` _pickupedactor))))

(fn `SetNextState`
  (bind _returnvalue (`|GenericCreateObject` "/Game/MartaHub/Blueprints/States/BP_EmptyHandsState.BP_EmptyHandsState_C" (`self.Owner`)))
  (`self.InitDataByState` _returnvalue self true))