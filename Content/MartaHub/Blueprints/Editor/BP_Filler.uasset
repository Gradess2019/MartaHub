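; BP_Filler is a construction-script actor that fills the line between StartLocation and EndLocation with randomly chosen static meshes.
; GetLastIndex derives the instance count from the distance at 50-unit spacing, and the script adds or trims Instances entries to match.
; SpawnStaticMeshActor creates each piece as a movable StaticMeshActor child actor, positioned by a normalized-direction math expression.
; Trimming and ClearInstances only edit the array, without destroying actors.
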(fn ConstructionScript
  (bind _returnvalue (CallFunction|GetLastIndex))
  (bind _instances (Variables|Editor|GetInstances))
  (bind _instances_2 (Variables|Editor|GetInstances))
  (bind _returnvalue_2 (Utilities|Array|LastIndex _instances))
  (bind _returnvalue_3 (Utilities|Array|LastIndex _instances_2))
  (if (> (Utilities|Array|Length (Variables|Editor|GetMeshes)) 0)
    (if (> _returnvalue_2 _returnvalue)
      (bind (_arrayindex _arrayelement) (Utilities|Array|ReverseforEachLoop _instances_2)
        (:LoopBody
          (if (> _arrayindex (- _returnvalue_3 (- _returnvalue_3 (CallFunction|GetLastIndex))))
            (Utilities|Array|RemoveItem (Variables|Editor|GetInstances) _arrayelement))))
      (elif (< _returnvalue_2 _returnvalue)
        (for _index (range 0 (- (CallFunction|GetLastIndex) (- (Utilities|Array|Length (Variables|Editor|GetInstances)) 1)))
          (bind (_actor _component) (CallFunction|SpawnStaticMeshActor (|({4EA991D7-47FD-1584-0736-C98A25DB734B}+(((Normalize(({8CD055E7-4533-64B6-775C-2E8C68085C0B}-{4EA991D7-47FD-1584-0736-C98A25DB734B})))*Offset)*Id)) 5e+01 _index)))
          (Utilities|Array|Add (Variables|Editor|GetInstances) _actor)
          (Components|StaticMesh|SetStaticMesh _component (Utilities|Array|Get(acopy) (Variables|Editor|GetMeshes) (Math|Random|RandomIntegerinRange 0 (Utilities|Array|LastIndex (Variables|Editor|GetMeshes))))))))))

(fn ClearInstances
  (Utilities|Array|Clear (Variables|Editor|GetInstances)))

(fn GetLastIndex
  (return (- (Math|Float|Round (/ (Math|Vector|Distance(Vector) (Variables|Editor|GetStartLocation) (Variables|Editor|GetEndLocation)) 5e+01)) 1)))

(fn SpawnStaticMeshActor
  (params (RelativeTransform_Location :type Vector))
  (bind _returnvalue (AddComponent|AddChildActorComponent true (Math|Transform|MakeTransform RelativeTransform_Location "0, 0, 0" "1,1,1")))
  (bind _output_get (LocalVariables|SetActorComponent _returnvalue))
  (ChildActorComponent|SetChildActorClass _output_get "/Script/Engine.StaticMeshActor")
  (Transformation|SetMobility (LocalVariables|GetActorComponent) "Movable")
  (Transformation|AttachComponentToComponent (LocalVariables|GetActorComponent) (Variables|Default|GetDefaultSceneRoot) "None" "KeepRelative" "KeepRelative" "KeepRelative" false)
  (bind _asstatic_mesh_actor (Utilities|Casting|CastToStaticMeshActor (Variables|/Script/Engine.ChildActorComponent|GetChildActor (LocalVariables|GetActorComponent))))
  (return _asstatic_mesh_actor (Variables|/Script/Engine.StaticMeshActor|GetStaticMeshComponent _asstatic_mesh_actor)))