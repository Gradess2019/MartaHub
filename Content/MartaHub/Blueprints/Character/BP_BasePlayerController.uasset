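; Base player controller that relays radio control requests from the player to the server.
; AdjustVolume and Play events each forward the target Radio and their argument to matching Server-prefixed events.
; Those events then call AdjustVolume or Play with a URL on the Radio actor, routing changes through the player-owned controller.
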(event `self.AdjustVolume`
  (params (Radio :type "Radio Object Reference") (Delta :type "Float (single-precision)"))
  (`self.ServerAdjustVolume` Radio Delta))

(event `ServerAdjustVolume`
  (params (Radio :type "Radio Object Reference") (Delta :type "Float (double-precision)" :default 0.05))
  (`Radio.AdjustVolume` Radio Delta))

(event `self.Play`
  (params (Radio :type "Radio Object Reference") (URL :type String))
  (`self.ServerPlay` Radio URL))

(event `ServerPlay`
  (params (Radio :type "Radio Object Reference") (URL :type String))
  (`Radio.Play` Radio URL))

(fn `UserConstructionScript`
  (`parent.UserConstructionScript`))