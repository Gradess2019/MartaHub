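; Base player character for MartaHub that handles head rotation, footstep audio, VSync setup and the game menu.
; On server or local instances it builds command objects, running VSync at start and menu creation on Menu press; other instances disable spring arm control rotation.
; The authority multicasts control rotation to the head each tick.
; It also runs a speed-gated looping timer that traces downward to choose wood, linoleum or glass footstep sounds.
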(event `self.ReceiveBeginPlay`
  (if (or (`KismetSystemLibrary.IsServer`) (`self.IsLocallyControlled`))
    (`self.InitCommands`)
    (bind _setvsynccommand (`self.SetVSyncCommand`)
      (:`then`
        (`BaseCommand.Execute` _setvsynccommand))
      (:`else`))
    (else
      (set `SpringArmComponent.bUsePawnControlRotation` false (`self.SpringArm`)))))

(event `PlayFootstepSound`
  (bind _returnvalue (`self.K2_GetActorLocation`))
  (bind _returnvalue_2 (`self.K2_GetActorLocation`))
  (bind _outhit (`KismetSystemLibrary.LineTraceSingle` _returnvalue (+ _returnvalue (* (`KismetMathLibrary.NegateVector` (`self.GetActorUpVector`)) 100.0)) "TraceTypeQuery1" true :!label _label))
  (switch `EPhysicalSurface` (`GameplayStatics.GetSurfaceType` _outhit)
    (:`SurfaceType1`
      (`GameplayStatics.PlaySoundAtLocation` "/Game/MartaHub/Sounds/Surface/A_TableSurface.A_TableSurface" _returnvalue_2 (struct) 1.0 1.0 0.0 null null null))
    (:`SurfaceType2`
      (`GameplayStatics.PlaySoundAtLocation` "/Game/MartaHub/Sounds/Surface/A_LinoleumSurface.A_LinoleumSurface" _returnvalue_2 (struct) 1.0 1.0 0.0 null null null))
    (:`SurfaceType4`
      (`GameplayStatics.PlaySoundAtLocation` "/Game/MartaHub/Sounds/Surface/A_GlassSurface.A_GlassSurface" _returnvalue_2 (struct) 1.0 1.0 0.0 null null null))))

(event `self.ReceiveTick`
  (params (DeltaSeconds :type "Float (single-precision)"))
  (bind _charactermovement (`self.CharacterMovement`))
  (`/Engine/EditorBlueprintResources/ActorMacros.Switch Has Authority`
    (:`Authority`
      (`self.Multicast_SetHeadRotation` (`self.GetControlRotation`))
      (if (and (`NavMovementComponent.IsMovingOnGround` _charactermovement) (> (`KismetMathLibrary.VSizeSquared` (`MovementComponent.Velocity` _charactermovement)) 27000.0))
        (if (not (`KismetSystemLibrary.K2_IsValidTimerHandle` (`self.FootstepTimer`)))
          (bind _returnvalue (`KismetSystemLibrary.K2_SetTimerDelegate` (delegate `PlayFootstepSound`) 0.5 true))
          (set `self.FootstepTimer` _returnvalue)
          (goto _label))
        (else
          (`KismetSystemLibrary.K2_ClearAndInvalidateTimerHandle` (`self.FootstepTimer`)))))))

(event `Multicast_SetHeadRotation`
  (params (NewRotation :type "Rotator Structure"))
  (`SceneComponent.K2_SetWorldRotation` (`self.Head`) NewRotation false false))

(event `InputAction|Menu`
  (params (Key :type "Key Structure"))
  (:`Pressed`
    (bind _createwidgetcommand (`self.CreateWidgetCommand`)
      (:`then`
        (`BaseCommand.Execute` _createwidgetcommand))
      (:`else`))))

(fn `InitCommands`
  (`self.InitSetVSyncCommand`)
  (`self.InitCreateWidgetCommand`))

(fn `InitCreateWidgetCommand`
  (bind _returnvalue (`|GenericCreateObject` "/Script/CommandPack.CreateWidgetCommand" self))
  (bind _returnvalue_2 (`CreateWidgetCommand.Init` _returnvalue (make `CreateWidgetCommandData` (`GameplayStatics.GetPlayerController` 0) "/Game/MartaHub/Blueprints/Widgets/WBP_GameMenu.WBP_GameMenu_C" true true true "DoNotLock" 0 "GameMenu")))
  (if _returnvalue_2
    (set `self.CreateWidgetCommand` _returnvalue)))

(fn `InitSetVSyncCommand`
  (bind _returnvalue (`|GenericCreateObject` "/Script/CommandPack.SetVSyncCommand" self))
  (bind _returnvalue_2 (`SetVSyncCommand.Init` _returnvalue (make `SetVSyncCommandData` true)))
  (if _returnvalue_2
    (set `self.SetVSyncCommand` _returnvalue)))

(fn `UserConstructionScript`
  (`parent.UserConstructionScript`))