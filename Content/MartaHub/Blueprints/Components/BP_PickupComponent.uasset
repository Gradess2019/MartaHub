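; Pickup component that handles interact and fire input through a state object pattern.
; On BeginPlay it constructs an empty-hands state and initializes it with itself as owner, with the update-owner flag set.
; Tick and the interact press, interact release and fire press events forward to the current state, which SetPickupState replaces.
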(event `self.ReceiveBeginPlay`
  (bind _returnvalue (`|GenericCreateObject` "/Game/MartaHub/Blueprints/States/BP_EmptyHandsState.BP_EmptyHandsState_C" self))
  (`/Game/MartaHub/Blueprints/States/BP_PickupStateBase.InitData` _returnvalue self null true))

(event `self.ReceiveTick`
  (params (DeltaSeconds :type "Float (single-precision)"))
  (message `Updatable.Update` (`self.State`) DeltaSeconds))

(event `self.PressInteract`
  (message `InputControllable.PressInteract` (`self.State`)))

(event `self.ReleaseInteract`
  (message `InputControllable.ReleaseInteract` (`self.State`)))

(event `self.PressFire`
  (message `InputControllable.PressFire` (`self.State`)))

(event `/Game/MartaHub/Blueprints/Interfaces/BPI_Pickuper.SetPickupState`
  (params (NewState :type "/Game/MartaHub/Blueprints/States/BP_PickupStateBase Object Reference"))
  (set `self.State` NewState))